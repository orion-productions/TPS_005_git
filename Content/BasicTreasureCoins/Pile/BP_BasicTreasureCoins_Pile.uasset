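; BP_BasicTreasureCoins_Pile is a placeable treasure coin pile whose look varies by a chosen metal type of copper, silver or gold.
; The construction script maps MetalType to a tint and writes it, along with a roughness adjustment, to the CoinPile component's default Custom Primitive Data.
; The event graph holds only disabled placeholder events, so it has no runtime logic.
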(event EventBeginPlay)

(event Collision|EventActorBeginOverlap
  (params (OtherActor :type Actor%20Object%20Reference)))

(event EventTick
  (params (DeltaSeconds :type Float%20%28single-precision%29)))

(fn ConstructionScript
  (Utilities|FlowControl|Sequence ; Then0: Determine tint color based on chosen MetalType\nThen1: Set Custom Primitive Data for color + roughness adjust
    (:then_0
      (switch name (Variables|Default|GetMetalType)
        (:Copper
          (Variables|Default|SetPrimData_Tint (Math|Vector4|MakeVector4 0.8 0.36 0.216 0.0)))
        (:Silver
          (Variables|Default|SetPrimData_Tint (Math|Vector4|MakeVector4 0.7 0.85 1.0 0.0)))
        (:Gold
          (Variables|Default|SetPrimData_Tint (Math|Vector4|MakeVector4 0.85 0.5 0.11 0.0)))))
    (:then_1
      (Rendering|Material|SetDefaultCustomPrimitiveDataVector4 (Variables|Default|GetCoinPile) 0 (Variables|Default|GetPrimData_Tint))
      (Rendering|Material|SetDefaultCustomPrimitiveDataFloat (Variables|Default|GetCoinPile) 4 (Variables|Default|GetRoughnessAdjust)))))